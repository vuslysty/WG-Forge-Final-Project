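; BP_EggTrough is a trough that spawns eggs and steps them along preset points for a catching game.
; Construction caches transforms of its placed egg components as the path, and difficulty's move time is divided across those points for each spawned egg.
; Eggs expose a move-next-point event for teleporting stepwise; at the path's end they are destroyed and EggInEndPosition reports the required catch pose.
; The pose check in EventGraph is disconnected.
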(fn `AddAllEggTransformsToArray`
  (`self.AddEggTransformToArray` (`self.BP_Egg`))
  (`self.AddEggTransformToArray` (`self.BP_Egg1`))
  (`self.AddEggTransformToArray` (`self.BP_Egg2`))
  (`self.AddEggTransformToArray` (`self.BP_Egg3`))
  (`self.AddEggTransformToArray` (`self.BP_Egg4`))
  (`self.AddEggTransformToArray` (`self.BP_Egg5`))
  (`self.AddEggTransformToArray` (`self.BP_Egg6`))
  (`self.AddEggTransformToArray` (`self.BP_Egg7`))
  (`self.AddEggTransformToArray` (`self.BP_Egg8`)))

(fn `AddEggTransformToArray`
  (params (EggComponent :type "ChildActorComponent Object Reference"))
  (`KismetArrayLibrary.Array_Add` (`self.EggTransforms`) (`SceneComponent.K2_GetComponentToWorld` EggComponent)))

(fn `MoveEggToNextPosition`
  (params (egg :type "/Game/Game/BP_Egg Object Reference"))
  (bind _egg (`local.egg`))
  ;[1 1 1] Increment egg position index
  (bind _output_get (set `/Game/Game/BP_Egg.PositionIndex` (+ (`/Game/Game/BP_Egg.PositionIndex` egg) 1) (`local.egg`)))
  (if (>= _output_get (`KismetArrayLibrary.Array_Length` (`self.EggTransforms`)))
    (`self.Remove Egg` (`local.egg`))
    (`self.EggInEndPosition` (`self.RequireCatchPose`))
    (else
      ;[1 1 1] Move egg to new position
      (`self.K2_SetActorTransform` _egg (`|GetArrayItem` (`self.EggTransforms`) (`/Game/Game/BP_Egg.PositionIndex` _egg)) false true))))

(fn `Remove All Eggs`
  (bind _result (`BlueprintSetLibrary.Set_ToArray` (`self.MoveEggs`)))
  (bind (_arrayindex _arrayelement) (`/Engine/EditorBlueprintResources/StandardMacros.ReverseForEachLoop` _result)
    (:`LoopBody`
      (clear `/Game/Game/BP_Egg.MoveNextPoint` _arrayelement)
      (`self.Remove Egg` _arrayelement))))

(fn `Remove Egg`
  (params (Egg :type "/Game/Game/BP_Egg Object Reference (by ref)"))
  (`BlueprintSetLibrary.Set_Remove` (`self.MoveEggs`) Egg)
  (`self.K2_DestroyActor` Egg))

(fn `SpawnEgg`
  (bind _returnvalue (`|SpawnActorFromClass` "/Game/Game/BP_Egg.BP_Egg_C" (`|GetArrayItem` (`self.EggTransforms`)) "Undefined" "OverrideRootScale" self null))
  (set `/Game/Game/BP_Egg.PositionIndex` 0 _returnvalue)
  (`BlueprintSetLibrary.Set_Add` (`self.MoveEggs`) _returnvalue)
  (add `/Game/Game/BP_Egg.MoveNextPoint` _returnvalue (`|CreateDelegate` :!event `MoveEggToNextPosition`))
  (bind _asmy_game_mode (cast `/Game/Game/My_GameMode` (`GameplayStatics.GetGameMode`)))
  (set `/Game/Game/BP_Egg.MoveTime` (/ (`.MoveEggTime_4_00ABF09E4204EAB8ACF8659E52E7462E` (break `/Game/Game/LevelDifficulty` (`/Game/Game/My_GameMode.CurrentDifficulty` _asmy_game_mode))) (`KismetMathLibrary.Conv_IntToDouble` (`KismetArrayLibrary.Array_Length` (`self.EggTransforms`)))) _returnvalue))

(fn `UserConstructionScript`
  (`self.AddAllEggTransformsToArray`))