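; BP_Character is the player character that switches between four catch poses (left/right, up/down), plus Idle and Defeat.
; Catch inputs set the pose and a held-key counter returns it to Idle when the last key is released.
; ChangePose fakes each facing by rotating the skeletal mesh and mirroring it with negative scale.
; Idle and Defeat use the previous pose, saved on full release, to choose mirroring.
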(event `InputAction|CatchRightUp`
  (params (Key :type "Key Structure"))
  (:`Pressed`
    (set `self.Pose` "NewEnumerator4")
    (set `self.CountOfPressedPoseKeys` (+ (`self.CountOfPressedPoseKeys`) 1) :!label _label)
    (`self.ChangePose` :!label _label_2))
  (:`Released`
    (bind _output_get (set `self.CountOfPressedPoseKeys` (- (`self.CountOfPressedPoseKeys`) 1) :!label _label_3))
    (if (== _output_get 0)
      (set `self.PrevPose` (`self.Pose`))
      (set `self.Pose` "NewEnumerator0")
      (goto _label_2))))

(event `InputAction|CatchRightDown`
  (params (Key :type "Key Structure"))
  (:`Pressed`
    (set `self.Pose` "NewEnumerator3")
    (goto _label))
  (:`Released`
    (goto _label_3)))

(event `InputAction|CatchLeftUp`
  (params (Key :type "Key Structure"))
  (:`Pressed`
    (set `self.Pose` "NewEnumerator2")
    (goto _label))
  (:`Released`
    (goto _label_3)))

(event `InputAction|CatchLeftDown`
  (params (Key :type "Key Structure"))
  (:`Pressed`
    (set `self.Pose` "NewEnumerator1")
    (goto _label))
  (:`Released`
    (goto _label_3)))

(event `ChangePose`
  (bind _skeletalmesh (`self.SkeletalMesh`))
  (bind _prevpose (`self.PrevPose`))
  (switch `/Game/MixamoAnimation/CharacterPose` (`self.Pose`)
    (:`NewEnumerator0`
      (`SceneComponent.K2_SetRelativeRotation` _skeletalmesh (struct :`Yaw` 90.0) false false :!label _label_4)
      (if (or (`|EnumEquality` _prevpose "NewEnumerator4") (`|EnumEquality` _prevpose "NewEnumerator3"))
        (`SceneComponent.SetRelativeScale3D` _skeletalmesh (-1.0 1.0 1.0))
        (else
          (`SceneComponent.SetRelativeScale3D` _skeletalmesh (1.0 1.0 1.0) :!label _label_5))))
    (:`NewEnumerator1`
      (`SceneComponent.K2_SetRelativeRotation` _skeletalmesh (struct :`Yaw` 90.0) false false)
      (goto _label_5))
    (:`NewEnumerator2`
      (`SceneComponent.K2_SetRelativeRotation` _skeletalmesh (struct) false false)
      (`SceneComponent.SetRelativeScale3D` _skeletalmesh (1.0 -1.0 1.0) :!label _label_6))
    (:`NewEnumerator3`
      (`SceneComponent.K2_SetRelativeRotation` _skeletalmesh (struct :`Yaw` -90.0) false false)
      (goto _label_6))
    (:`NewEnumerator4`
      (`SceneComponent.K2_SetRelativeRotation` :`self` _skeletalmesh)
      (goto _label_5))
    (:`NewEnumerator5`
      (goto _label_4))))

(fn `UserConstructionScript`)